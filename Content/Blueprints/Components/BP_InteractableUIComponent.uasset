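; BP_InteractableUIComponent is a player character component that shows a world-space indicator on the first nearby interactable.
; On BeginPlay it spawns a hidden widget holder actor and binds to the character's interactables update, which moves the holder onto the target or hides it.
; While visible, Tick yaws the widget toward the camera by flattening Z and fills a progress bar from the target's GetProgressMessage, shown only above zero.
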(event `self.ReceiveBeginPlay`
  (bind _asbp_player_character (cast `/Game/Blueprints/GameModeBases/BP_PlayerCharacter` (`self.GetOwner`))
    (:`then`
      (bind _output_get (set `self.PC` _asbp_player_character))
      (add `/Game/Blueprints/GameModeBases/BP_PlayerCharacter.OnInteractablesUpdate` _output_get (delegate `UpdateInteractables`))
      (bind _returnvalue (`|SpawnActorFromClass` "/Game/UI/Interactables/BP_InteractableWidgetHolder.BP_InteractableWidgetHolder_C" (`KismetMathLibrary.MakeTransform` (0.0 0.0 0.0)) "Undefined" "MultiplyWithRoot" null null))
      (bind _output_get_2 (set `self.InteractWidgetHolder` _returnvalue))
      (bind _widget (`/Game/UI/Interactables/BP_InteractableWidgetHolder.Widget` _output_get_2))
      (`Widget.SetVisibility` (`WidgetComponent.GetWidget` _widget) "Hidden")
      (`PrimitiveComponent.SetCastShadow` _widget false))
    (:`CastFailed`
      (`self.SetActive` false))))

(event `UpdateInteractables`
  (bind _interactwidgetholder (`self.InteractWidgetHolder`))
  (if (`KismetArrayLibrary.Array_IsNotEmpty` (`/Game/Blueprints/GameModeBases/BP_PlayerCharacter.NearbyInteractables` (`self.PC`)))
    (bind _asactor (cast `Actor` (`KismetSystemLibrary.Conv_InterfaceToObject` (`|GetArrayItem` (`/Game/Blueprints/GameModeBases/BP_PlayerCharacter.NearbyInteractables` (`self.PC`))))))
    (bind _output_get (set `self.InteractTarget` _asactor))
    (`Actor.K2_SetActorLocation` _interactwidgetholder (`Actor.K2_GetActorLocation` _output_get) false false)
    (`Widget.SetVisibility` (`WidgetComponent.GetWidget` (`/Game/UI/Interactables/BP_InteractableWidgetHolder.Widget` _interactwidgetholder)) "Visible")
    (else
      (`Widget.SetVisibility` (`WidgetComponent.GetWidget` (`/Game/UI/Interactables/BP_InteractableWidgetHolder.Widget` (`self.InteractWidgetHolder`))) "Hidden"))))

(event `self.ReceiveTick`
  (params (DeltaSeconds :type "Float (single-precision)"))
  (switch `ESlateVisibility` (`Widget.GetVisibility` (`WidgetComponent.GetWidget` (`/Game/UI/Interactables/BP_InteractableWidgetHolder.Widget` (`self.InteractWidgetHolder`))))
    (:`Visible`
      (`self.RotateTowardsPlayer`)
      (`self.UpdateProgress`))))

(fn `RotateTowardsPlayer`
  (`SceneComponent.K2_SetWorldRotation` (`/Game/UI/Interactables/BP_InteractableWidgetHolder.Widget` (`self.InteractWidgetHolder`)) (`KismetMathLibrary.FindLookAtRotation` (* (`SceneComponent.K2_GetComponentLocation` (`/Game/UI/Interactables/BP_InteractableWidgetHolder.Widget` (`self.InteractWidgetHolder`))) (1.0 1.0 0.0)) (* (`SceneComponent.K2_GetComponentLocation` (`/Game/Blueprints/GameModeBases/BP_PlayerCharacter.Camera` (`self.PC`))) (1.0 1.0 0.0))) false false))

(fn `UpdateProgress`
  (bind _asbp_interactable_indicator (cast `/Game/UI/Interactables/BP_InteractableIndicator` (`WidgetComponent.GetWidget` (`/Game/UI/Interactables/BP_InteractableWidgetHolder.Widget` (`self.InteractWidgetHolder`)))))
  (bind _progress (message `/Game/Blueprints/Interfaces/BPI_Interact.GetProgress` (`self.InteractTarget`)))
  (bind _progress_2 (`/Game/UI/Interactables/BP_InteractableIndicator.Progress` _asbp_interactable_indicator))
  (`ProgressBar.SetPercent` _progress_2 _progress)
  (if (> _progress 0.0)
    (`Widget.SetVisibility` _progress_2 "Visible")
    (else
      (`Widget.SetVisibility` _progress_2 "Hidden"))))