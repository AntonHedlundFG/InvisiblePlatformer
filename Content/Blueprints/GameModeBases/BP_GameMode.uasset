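; Game mode for a two-player game that holds the game state paused until both players log in and assigns platform actors to their pawns.
; PostLogin collects controllers; from the second login it waits briefly, applies platform ownership, then clears IsPaused on BP_GameState.
; RegisterPlatform sets a platform's owner immediately if both players are present, otherwise queues it by player index in OwnerVisibleActors for SetPlatformOwnerships.
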(event `self.K2_PostLogin`
  (params (NewPlayer :type "PlayerController Object Reference"))
  (bind _playercontrollers (`self.PlayerControllers`))
  (`KismetArrayLibrary.Array_Add` _playercontrollers NewPlayer)
  (if (>= (`KismetArrayLibrary.Array_Length` _playercontrollers) 2)
    (`KismetSystemLibrary.Delay` 5.0)
    (`self.SetPlatformOwnerships`)
    (bind _asbp_game_state (cast `/Game/Blueprints/GameModeBases/BP_GameState` (`GameplayStatics.GetGameState`)))
    (set `/Game/Blueprints/GameModeBases/BP_GameState.IsPaused` false _asbp_game_state)))

(event `self.ReceiveBeginPlay`
  (bind _asbp_game_state (cast `/Game/Blueprints/GameModeBases/BP_GameState` (`GameplayStatics.GetGameState`)))
  (set `/Game/Blueprints/GameModeBases/BP_GameState.IsPaused` true _asbp_game_state))

(fn `RegisterPlatform`
  (params (TargetActor :type "Actor Object Reference") (`Player ID` :type Integer))
  (if (>= (`KismetArrayLibrary.Array_Length` (`self.PlayerControllers`)) 2)
    (`self.SetOwner` TargetActor (`Controller.K2_GetPawn` (`|GetArrayItem` (`self.PlayerControllers`) `Player ID`)))
    (`self.SetOwner` TargetActor (`Controller.K2_GetPawn` (`|GetArrayItem` (`self.PlayerControllers`) `Player ID`)))
    (else
      (`BlueprintMapLibrary.Map_Add` (`self.OwnerVisibleActors`) TargetActor (`KismetMathLibrary.Clamp` `Player ID` 0 1)))))

(fn `SetPlatformOwnerships`
  (bind _ownervisibleactors (`self.OwnerVisibleActors`))
  (bind _keys (`BlueprintMapLibrary.Map_Keys` _ownervisibleactors))
  (for _array_element _keys
    (`self.SetOwner` _array_element (`Controller.K2_GetPawn` (`|GetArrayItem` (`self.PlayerControllers`) (`BlueprintMapLibrary.Map_Find` _ownervisibleactors _array_element))))))

(fn `UserConstructionScript`)